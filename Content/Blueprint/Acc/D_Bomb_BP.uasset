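; A bomb Actor Blueprint that explodes when its capsule hits something or drops below world height zero.
; The explosion spawns an emitter, plays a sound, and applies damage to the single actor found by a large-radius sphere trace, drawn for debugging.
; A hit also destroys the actor after a short delay, while the height check on Tick repeats the explosion every frame without destroying it.
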(event `self.ReceiveTick`
  (params (DeltaSeconds :type "Float (single-precision)"))
  (bind _returnvalue (`SceneComponent.K2_GetComponentLocation` (`self.Capsule`)))
  (if (< (.z _returnvalue) 0.0)
    (`GameplayStatics.SpawnEmitterAtLocation` "/Game/Particles/Explosion.Explosion" _returnvalue :!label _label)
    (`GameplayStatics.PlaySoundAtLocation` null _returnvalue (struct) 2.0 1.0 0.0 null null null null)
    (bind _outhit (`KismetSystemLibrary.SphereTraceSingle` :`Start` _returnvalue :`End` _returnvalue :`Radius` 2000.0 :`TraceChannel` "TraceTypeQuery1" :`DrawDebugType` "ForOneFrame"))
    (`GameplayStatics.ApplyDamage` (`.HitActor` (`GameplayStatics.BreakHitResult` _outhit)) 1000.0)))

(event `self.Capsule.OnComponentHit`
  (params (HitComponent :type "PrimitiveComponent Object Reference") (OtherActor :type "Actor Object Reference") (OtherComp :type "PrimitiveComponent Object Reference") (NormalImpulse :type "Vector Structure") (Hit :type "HitResult Structure (by ref)"))
  (`|ExecutionSequence`
    (:`then_0`
      (goto _label))
    (:`then_1`
      (`KismetSystemLibrary.Delay` 1.0)
      (`self.K2_DestroyActor`))))

(fn `UserConstructionScript`)