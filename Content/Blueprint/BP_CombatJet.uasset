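; Player-controlled combat jet that taxis, takes off, flies, lands, drops bombs and interacts with quest actors.
; A Flying flag switches inputs between ground and flight handling, with interpolation smoothing movement, exhaust and engine audio.
; Space at speed triggers takeoff; a downward trace lands it at low speed.
; Tick also drains MaxHeath as fuel and sphere-traces for IInteraction targets; Supplies spawns the same Bomba as FireMissile, and Death only prints.
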(event `Key|E`
  (params (Key :type "Key Structure"))
  ;[1 0.7157 0] Luiz Parte
  (:`Pressed`
    (if (`self.drop`)
      (`KismetSystemLibrary.PrintString` "Esta sem a Bomba")
      (set `self.drop` false)
      (else
        (`KismetSystemLibrary.PrintString` "Esta com a Bomba")
        (set `self.drop` true)))))

(event `Death`
  ;[1 0.7157 0] Luiz Parte
  (`KismetSystemLibrary.PrintString` "YOU DIED"))

(event `DecayGas`
  ;[1 0.7157 0] Luiz Parte
  ;;[1 1 1] Sistema de Gas
  (if (not (<= (`self.Max Heath`) 0.0))
    (`KismetSystemLibrary.Delay` 0.01)
    (if (`self.MotorLigado`)
      (bind _output_get (set `self.Max Heath` (- (`self.Max Heath`) 0.01)))
      (`KismetSystemLibrary.PrintString` (`KismetStringLibrary.Conv_DoubleToString` _output_get)))))

(event `SetGas`
  ;[1 0.7157 0] Luiz Parte
  ;;[1 1 1] Sistema de Gas
  (set `self.CurrentHealth` (`self.Max Heath`)))

(event `InputAction|FireMissile`
  (params (Key :type "Key Structure"))
  (bind (_returnvalue_x _returnvalue_y) (`KismetMathLibrary.BreakVector` (`self.K2_GetActorLocation`)))
  ;[1 1 1] Drop Bomb
  (:`Pressed`
    (if (`self.Flying?`)
      (`|SpawnActorFromClass` "/Game/Drops/Bomba.Bomba_C" (`KismetMathLibrary.MakeTransform` (`KismetMathLibrary.MakeVector` _returnvalue_x (- _returnvalue_y 75.0))) "Undefined" "MultiplyWithRoot" null null))))

(event `InputAction|Supplies`
  (params (Key :type "Key Structure"))
  (bind (_returnvalue_x _returnvalue_y) (`KismetMathLibrary.BreakVector` (`self.K2_GetActorLocation`)))
  ;[1 1 1] Drop Supplies
  (:`Pressed`
    (if (`self.Flying?`)
      (`|SpawnActorFromClass` "/Game/Drops/Bomba.Bomba_C" (`KismetMathLibrary.MakeTransform` (`KismetMathLibrary.MakeVector` _returnvalue_x (- _returnvalue_y 75.0))) "Undefined" "MultiplyWithRoot" null null))))

(event `InputAction|Interact`
  (params (Key :type "Key Structure"))
  ;[1 1 1] Quest Giver Interaction
  (:`Pressed`
    (bind _lookatactor (`self.LookAtActor`)
      (:`then`
        (bind _objectiveid (message `/Game/QuestSystem/IInteraction.InteractWith` _lookatactor))
        (`self.OnObjectiveIdCalled` _objectiveid))
      (:`else`))))

(event `self.ReceiveBeginPlay`
  ;[0 0 0] Event BeginPlay
  (`self.SetGas`)
  (`|ExecutionSequence`
    (:`then_0`
      _)
    (:`then_1`
      ;;[1 1 1] Scale of Exhaust
      (`SceneComponent.SetRelativeScale3D` (`self.LeftExhaust`) (0.0 0.0 0.0))
      (`SceneComponent.SetRelativeScale3D` (`self.RightExhaust`) (0.0 0.0 0.0))))
  ;;[1 1 1] Fly at Minimum Speed
  (set `self.Target Speed` (`self.Minimum Speed`))
  (set `self.StartZOffset` 150.0)
  (bind _returnvalue (`|CreateWidget` "/Game/Blueprint/UI/WBP_PlayerHUD.WBP_PlayerHUD_C"))
  (`UserWidget.AddToViewport` _returnvalue 0))

(event `self.ReceiveTick`
  (params (DeltaSeconds :type "Float (single-precision)"))
  (bind _jetengineaudio (`self.JetEngineAudio`))
  (bind _returnvalue (`KismetMathLibrary.NormalizeToRange` (`self.Current Speed`) 0.0 (`self.Maximum Speed`)))
  ;[0 0 0] Event TICK
  (`|ExecutionSequence`
    (:`then_0`
      (`self.DecayGas`)
      (`|ExecutionSequence`
        (:`then_0`
          ;;[1 1 1] Speed Up gradually
          (bind _output_get (set `self.MoveForwardINTER` (`KismetMathLibrary.FClamp` (`KismetMathLibrary.FInterpTo` (stale _output_get) (`self.GetInputAxisValue`) (`GameplayStatics.GetWorldDeltaSeconds`) 0.2))))
          (`SceneComponent.SetRelativeScale3D` (`self.LeftExhaust`) (`KismetMathLibrary.VInterpTo` (`SceneComponent.RelativeScale3D` (`self.RightExhaust`)) (`KismetMathLibrary.SelectVector` (`KismetMathLibrary.MakeVector` _returnvalue _returnvalue _returnvalue) (0.0 0.0 0.0) (`self.Flying?`)) (`GameplayStatics.GetWorldDeltaSeconds`) (`KismetMathLibrary.SelectFloat` 4.0 0.5 (`self.Flying?`))))
          (`SceneComponent.SetRelativeScale3D` (`self.RightExhaust`) (`KismetMathLibrary.VInterpTo` (`SceneComponent.RelativeScale3D` (`self.RightExhaust`)) (`KismetMathLibrary.SelectVector` (`KismetMathLibrary.MakeVector` _returnvalue _returnvalue _returnvalue) (0.0 0.0 0.0) (`self.Flying?`)) (`GameplayStatics.GetWorldDeltaSeconds`) (`KismetMathLibrary.SelectFloat` 4.0 0.5 (`self.Flying?`))))
          (`AudioComponent.SetVolumeMultiplier` _jetengineaudio (`KismetMathLibrary.FInterpTo` (`AudioComponent.VolumeMultiplier` _jetengineaudio) (`KismetMathLibrary.SelectFloat` 1.0 (/ (`self.MoveForwardINTER`) 2.0) (`self.Flying?`)) (`GameplayStatics.GetWorldDeltaSeconds`) 3.0)))
        (:`then_1`
          ;;[1 1 1] If flying
          (if (`self.Flying?`)
            (`self.Add flight Movement`)
            (`self.Landing Trace` "ForOneFrame" (`self.StartZOffset`))))))
    (:`then_1`
      (`self.InteractTrace`))))

(event `InputAxis|MoveForward`
  (params (AxisValue :type "Float (single-precision)"))
  (bind _wheel_rotation_side_max (`self.Wheel Rotation Side Max`))
  (bind (_wheel_rotation_roll _wheel_rotation_pitch _wheel_rotation_yaw) (`KismetMathLibrary.BreakRotator` (`self.Wheel Rotation`)))
  (bind _aileron_rotation_max (`self.Aileron Rotation Max`))
  (bind _jetengineaudio (`self.JetEngineAudio`))
  (bind (_returnvalue_roll _returnvalue_pitch) (`KismetMathLibrary.BreakRotator` (`SceneComponent.GetSocketRotation` (`self.SK_West_Fighter_Typhoon`) "front_wheel_jnt")))
  ;[0.03346 0.2656 0] Move Forward
  (if (`self.Flying?`)
    (bind _output_get (set `self.Target Speed` (`KismetMathLibrary.FClamp` (+ (* AxisValue (`GameplayStatics.GetWorldDeltaSeconds`) 2500.0) (`self.Target Speed`)) (`self.Minimum Speed`) (`self.Maximum Speed`))))
    (`AudioComponent.SetPitchMultiplier` _jetengineaudio (`KismetMathLibrary.FInterpTo` (`AudioComponent.PitchMultiplier` _jetengineaudio) (`KismetMathLibrary.MapRangeClamped` _output_get (`self.Minimum Speed`) (`self.Maximum Speed`) 1.0 (`KismetMathLibrary.SelectFloat` 2.0 1.5 (`self.Flying?`))) (`GameplayStatics.GetWorldDeltaSeconds`) 3.0)))
  (if (not (`self.Flying?`))
    (`|ExecutionSequence`
      (:`then_0`
        (`self.K2_AddActorWorldOffset` (`KismetMathLibrary.MakeVector` (.x (* (`self.GetActorForwardVector`) (`self.MoveForwardINTER`) (/ (`self.Target Speed`) 500.0))) (.y (* (`self.GetActorForwardVector`) (`self.MoveForwardINTER`) (/ (`self.Target Speed`) 500.0)))) true)
        ;;[1 1 1] It will fly if have speed enough and pressing space
        (if (and (> (`self.MoveForwardINTER`) 0.7) (`PlayerController.IsInputKeyDown` (`GameplayStatics.GetPlayerController` 0) "SpaceBar"))
          (set `self.Flying?` true)
          (set `SpringArmComponent.bUsePawnControlRotation` false (`self.SpringArm`))
          (`self.K2_AddActorWorldOffset` (0.0 0.0 25.0) true)
          (set `self.Aileron Interior Rotation` (`KismetMathLibrary.MakeRotator` 0.0 (`KismetMathLibrary.MapRangeClamped` (`self.Flight Pitch`) -1.0 1.0 _aileron_rotation_max (* _aileron_rotation_max -1.0))))))
      (:`then_1`
        ;;[1 1 1] Wheel Rotation
        (set `self.Wheel Rotation` (`KismetMathLibrary.MakeRotator` 0.0 (+ _returnvalue_pitch (* (`self.MoveForwardINTER`) -500.0)) (`KismetMathLibrary.FInterpTo` _wheel_rotation_yaw (`KismetMathLibrary.MapRangeClamped` (`self.GetInputAxisValue`) -1.0 1.0 (* _wheel_rotation_side_max -1.0) _wheel_rotation_side_max) (`GameplayStatics.GetWorldDeltaSeconds`) 0.4)))))))

(event `InputAxis|LookUp`
  (params (AxisValue :type "Float (single-precision)"))
  (bind _returnvalue (`GameplayStatics.GetWorldDeltaSeconds`))
  (bind _back_rudder_rotation_max (`self.Back Rudder Rotation Max`))
  (bind _returnvalue_2 (* AxisValue (`KismetMathLibrary.SelectFloat` -1.0 1.0 (`self.Invert Vertical Flight?`))))
  ;[0.03346 0.2656 0] Look Up
  (if (`self.Flying?`)
    (bind _output_get (set `self.Flight Pitch` (`KismetMathLibrary.FInterpTo` (stale _output_get) _returnvalue_2 _returnvalue 10.0)))
    (`self.K2_AddActorLocalRotation` (`KismetMathLibrary.MakeRotator` 0.0 (* _output_get _returnvalue (`self.Flight Turn Rate`))))
    (set `self.Back Rudder Rotation` (`KismetMathLibrary.MakeRotator` 0.0 0.0 (`KismetMathLibrary.MapRangeClamped` (`self.Flight Turn`) -1.0 1.0 _back_rudder_rotation_max (* _back_rudder_rotation_max -1.0))))
    (else
      (`self.AddControllerPitchInput` _returnvalue_2))))

(event `InputAxis|Turn`
  (params (AxisValue :type "Float (single-precision)"))
  (bind _returnvalue (`GameplayStatics.GetWorldDeltaSeconds`))
  ;[0.03346 0.2656 0] Turn
  (if (`self.Flying?`)
    (bind _output_get (set `self.Flight Turn` (`KismetMathLibrary.FInterpTo` (stale _output_get) AxisValue _returnvalue 10.0)))
    (`self.K2_AddActorLocalRotation` (`KismetMathLibrary.MakeRotator` 0.0 0.0 (* _output_get _returnvalue (`self.Flight Turn Rate`))))
    (else
      (`self.AddControllerYawInput` AxisValue))))

(event `InputAxis|MoveRight`
  (params (AxisValue :type "Float (single-precision)"))
  (bind _aileron_rotation_max (`self.Aileron Rotation Max`))
  (bind _aileron_rotation_max_2 (`self.Aileron Rotation Max`))
  ;[0.03346 0.2656 0] Move Right/Left input
  (if (`self.Flying?`)
    (bind _output_get (set `self.Flight Roll` (`KismetMathLibrary.FInterpTo` (stale _output_get) AxisValue (`GameplayStatics.GetWorldDeltaSeconds`) 10.0)))
    (`self.K2_AddActorLocalRotation` (`KismetMathLibrary.MakeRotator` (* _output_get (`GameplayStatics.GetWorldDeltaSeconds`) 90.0)))
    (set `self.Aileron Flap Rotation Left` (`KismetMathLibrary.MakeRotator` 0.0 (`KismetMathLibrary.MapRangeClamped` (`self.GetInputAxisValue`) -1.0 1.0 _aileron_rotation_max_2 (* _aileron_rotation_max_2 -1.0))))
    (set `self.Aileron Flap Rotation Right` (`KismetMathLibrary.MakeRotator` 0.0 (`KismetMathLibrary.MapRangeClamped` (`self.GetInputAxisValue`) -1.0 1.0 (* _aileron_rotation_max -1.0) _aileron_rotation_max)))
    (elif (> (`self.GetInputAxisValue`) 0.0)
      (`self.K2_AddActorWorldRotation` (`KismetMathLibrary.MakeRotator` 0.0 0.0 (* AxisValue (`GameplayStatics.GetWorldDeltaSeconds`) 1.2))))))

(fn `Add flight Movement`
  (bind _returnvalue (`GameplayStatics.GetWorldDeltaSeconds`))
  ;[1 1 1] Flight Speed
  (bind _output_get (set `self.Current Speed` (`KismetMathLibrary.FInterpTo` (stale _output_get) (`self.Target Speed`) _returnvalue 8.0)))
  ;[1 1 1] Add movement in forward direction
  (`self.K2_AddActorWorldOffset` (* (`SceneComponent.GetForwardVector` (`self.SK_West_Fighter_Typhoon`)) (* _output_get _returnvalue)) true))

(fn `InteractTrace`
  (bind _returnvalue (`self.K2_GetActorLocation`))
  (bind (_outhit _returnvalue_2) (`KismetSystemLibrary.SphereTraceSingle` _returnvalue (+ _returnvalue (* (`self.GetActorForwardVector`) 100.0)) 20.0 "TraceTypeQuery2" false (`|MakeArray` (`self.GetOwner`))))
  (if _returnvalue_2
    (bind (_bblockinghit _binitialoverlap _time _distance _location _impactpoint _normal _impactnormal _physmat _hitactor) (`GameplayStatics.BreakHitResult` _outhit))
    (if (`KismetSystemLibrary.DoesImplementInterface` _hitactor "/Game/QuestSystem/IInteraction.IInteraction_C")
      (bind _output_get (set `self.LookAtActor` _hitactor))
      (message `/Game/QuestSystem/IInteraction.LookAt` _output_get)
      (else
        (set `self.LookAtActor` null)))
    (else
      (set `self.LookAtActor` null))))

(fn `Landing Trace`
  (params (Debug :type "EDrawDebugTrace Enum" :default "None") (SpawnedZOffset :type "Float (double-precision)"))
  (bind _returnvalue (`self.K2_GetActorLocation`))
  (bind (_returnvalue_roll _returnvalue_pitch _returnvalue_yaw) (`KismetMathLibrary.BreakRotator` (`self.K2_GetActorRotation`)))
  (bind (_outhit _returnvalue_2) (`KismetSystemLibrary.LineTraceSingle` _returnvalue (- _returnvalue (`KismetMathLibrary.MakeVector` 0.0 0.0 SpawnedZOffset)) "TraceTypeQuery1" false (`|MakeArray` self :!type "Actor Object Reference") Debug))
  (if _returnvalue_2
    (if (< (`KismetMathLibrary.MapRangeClamped` (`self.Target Speed`) (`self.Minimum Speed`) (`self.Maximum Speed`) 0.0 1.0) 0.5)
      (set `self.Flying?` false)
      (`self.K2_SetActorRelativeTransform` (`KismetMathLibrary.MakeTransform` (`KismetMathLibrary.VInterpTo` (`self.K2_GetActorLocation`) (+ (`.TraceEnd` (`GameplayStatics.BreakHitResult` _outhit)) (`KismetMathLibrary.MakeVector` 0.0 0.0 (`local.SpawnedZOffset`))) (`GameplayStatics.GetWorldDeltaSeconds`) 3.0) (`KismetMathLibrary.MakeRotator` 0.0 0.0 _returnvalue_yaw)))
      (set `SpringArmComponent.bUsePawnControlRotation` true (`self.SpringArm`))
      (set `self.MoveForwardINTER` 1.0))))

(fn `SetCameraLag`
  (bind _springarm (`self.SpringArm`))
  (bind _returnvalue (`KismetMathLibrary.SelectFloat` 10.0 5000000.0 (`self.Flying?`)))
  (set `SpringArmComponent.CameraLagSpeed` _returnvalue _springarm)
  (set `SpringArmComponent.CameraRotationLagSpeed` _returnvalue _springarm))

(fn `UserConstructionScript`)