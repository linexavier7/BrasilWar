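; BP_Plane is a plane Blueprint with a bomb toggle, a gas system and a player HUD.
; BeginPlay copies MaxHealth to CurrentHealth and shows WBP_PlayerHUD, while the E key flips the Drop flag with a debug message.
; DecayGas re-calls itself after short delays, draining MaxHealth as fuel while MotorLigado is true, and calls Death, which only prints, at zero.
; Nothing in this graph starts DecayGas.
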(event `Key|E`
  (params (Key :type "Key Structure"))
  (:`Pressed`
    (if (`self.drop`)
      (`KismetSystemLibrary.PrintString` "Esta sem a Bomba")
      (set `self.drop` false)
      (else
        (`KismetSystemLibrary.PrintString` "Esta com a Bomba")
        (set `self.drop` true)))))

(event `Death`
  (`KismetSystemLibrary.PrintString` "YOU DIED"))

(event `DecayGas`
  ;[1 1 1] Sistema de Gas
  (if (<= (`self.MaxHealth`) 0.0)
    (`self.Death`)
    (else
      (`KismetSystemLibrary.Delay` 0.01)
      (if (`self.MotorLigado`)
        (bind _output_get (set `self.MaxHealth` (- (`self.MaxHealth`) 0.01)))
        (`self.DecayGas`)))))

(event `self.ReceiveBeginPlay`
  ;[1 1 1] Sistema de Gas
  (set `self.CurrentHealth` (`self.MaxHealth`))
  (bind _returnvalue (`|CreateWidget` "/Game/Blueprint/UI/WBP_PlayerHUD.WBP_PlayerHUD_C"))
  (bind _output_get (set `self.Player HUD_ref` _returnvalue))
  (`UserWidget.AddToViewport` _output_get 0))

(fn `UserConstructionScript`)