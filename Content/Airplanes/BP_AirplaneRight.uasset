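; BP_AirplaneRight is a player-controlled airplane pawn that flies on axis input and fires missiles.
; On BeginPlay it takes over the first player's camera view.
; Forward input offsets the Frame component along local Y without sweep, vertical input adds movement along its up vector, and turn input adds controller yaw plus actor local pitch rotation.
; FireMissile spawns a BP_Missile at the Muzzle's location and rotation.
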(event `InputAxis|MoveForward`
  (params (AxisValue :type "Float (single-precision)"))
  ;[1 0.59 0.5501] Move Forward and Backwards
  (if true
    (`SceneComponent.K2_AddLocalOffset` (`self.Frame`) (`KismetMathLibrary.MakeVector` 0.0 AxisValue) false false)))

(event `self.ReceiveBeginPlay`
  ;[0.9301 0.8879 0.3372] Camera
  (`PlayerController.SetViewTargetWithBlend` (`PlayerState.GetPlayerController` (`Pawn.PlayerState` (`GameplayStatics.GetPlayerPawn` 0))) self 0.0 "VTBlend_Linear" 0.0 false))

(event `InputAxis|MoveUp`
  (params (AxisValue :type "Float (single-precision)"))
  ;[1 0.7178 0.5015] Move Up and Down
  (if true
    (`self.AddMovementInput` (`SceneComponent.GetUpVector` (`self.Frame`)) (`KismetMathLibrary.MultiplyByPi` AxisValue))))

(event `InputAxis|TurnRightandLeft`
  (params (AxisValue :type "Float (single-precision)"))
  (bind _returnvalue (`KismetMathLibrary.MultiplyByPi` AxisValue))
  ;[0.7146 1 0.6308] Turn Right or Left
  (if true
    (`self.AddControllerYawInput` _returnvalue)
    (`self.K2_AddActorLocalRotation` (`KismetMathLibrary.MakeRotator` 0.0 _returnvalue))))

(event `InputAction|FireMissile`
  (params (Key :type "Key Structure"))
  ;[1 0.928 0.4582] Missile
  (:`Pressed`
    (`|SpawnActorFromClass` "/Game/Blueprint/BP_Missile.BP_Missile_C" (`KismetMathLibrary.MakeTransform` (`SceneComponent.K2_GetComponentLocation` (`self.Muzzle`)) (`SceneComponent.K2_GetComponentRotation` (`self.Muzzle`))) "Undefined" "MultiplyWithRoot" null null)))

(fn `UserConstructionScript`)